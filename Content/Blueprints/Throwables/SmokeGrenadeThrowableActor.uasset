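; Throwable smoke grenade actor that flies as a projectile, then releases a smoke cloud.
; On spawn it orients against its velocity and tumbles by a random per-tick rotation until a sphere hit switches the mesh to physics simulation.
; A short timer spawns an enlarged smoke emitter at the mesh's location, then removes both the emitter and the actor after a delay.
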(event OnComponentHit(SphereComponent)
  (params (HitComponent :type Primitive%20Component%20Object%20Reference) (OtherActor :type Actor%20Object%20Reference) (OtherComp :type Primitive%20Component%20Object%20Reference) (NormalImpulse :type Vector :default "0, 0, 0") (Hit :type Hit%20Result%20Structure%20%28by%20ref%29))
  (Physics|SetSimulatePhysics (Variables|Default|GetStaticMeshComponent) true))

(event Custom|AfterDelay
  (bind _returnvalue (Effects|SpawnEmitteratLocation "/Game/Realistic_Starter_VFX_Pack_Vol2/Particles/Smoke/P_Smoke_A.P_Smoke_A" (Transformation|GetWorldLocation (Variables|Default|GetStaticMeshComponent)) "0, 0, 0" "5.000000,5.000000,5.000000"))
  (Utilities|FlowControl|Delay 5.0)
  (Components|DestroyComponent _returnvalue)
  (Actor|DestroyActor))

(event EventBeginPlay
  (Utilities|Time|SetTimerbyEvent (delegate Custom|AfterDelay) 2.0)
  (Transformation|SetActorRotation (Math|Rotator|MakeRotfromY (* (Variables|/Script/Engine.MovementComponent|GetVelocity (Variables|Default|GetProjectileMovementComp)) -1.0)))
  (Variables|Default|SetRandValue (Math|Random|RandomFloatinRange -2.0 2.0)))

(event EventTick
  (params (DeltaSeconds :type Float%20%28single-precision%29))
  (bind _randvalue (Variables|Default|GetRandValue))
  (if (not (Physics|IsSimulatingPhysics (Variables|Default|GetStaticMeshComponent) "None"))
    (Class|Actor|AddActorWorldRotation (Math|Rotator|MakeRotator _randvalue _randvalue _randvalue))))

(fn ConstructionScript)