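; Thrown Molotov actor that spins in flight and leaves a temporary burning area where it hits anything other than the player pawn.
; On overlap it stops, hides its visuals and spawns explosion and fire emitters, destroying itself after a randomized delay.
; While burning, each Tick sphere-traces for pawns and applies the GAS fire damage effect to those with an unblocked line trace to the impact point.
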(event OnComponentBeginOverlap(SphereComponent)
  (params (OverlappedComponent :type Primitive%20Component%20Object%20Reference) (OtherActor :type Actor%20Object%20Reference) (OtherComp :type Primitive%20Component%20Object%20Reference) (OtherBodyIndex :type Integer) (bFromSweep :type Boolean) (SweepResult :type Hit%20Result%20Structure%20%28by%20ref%29))
  (bind _projectilemovementcomp (Variables|Default|GetProjectileMovementComp))
  (if (!= OtherActor (Game|Player|GetPlayerPawn 0))
    (Variables|Default|SetSweep%20Result%20Location (.location SweepResult))
    (Components|Movement|StopMovementImmediately _projectilemovementcomp)
    (Game|Components|ProjectileMovement|StopSimulating _projectilemovementcomp (Collision|MakeHitResult false false 0.0 0.0 "0, 0, 0" "0, 0, 0" "0,0,1" "0,0,1" 0 0 0 "None" "None" 0 0 0 "0, 0, 0" "0, 0, 0"))
    (Development|SetHiddeninGame (Variables|Default|GetStaticMeshComponent) true false)
    (CallFunction|SpawnEmitter)
    (Collision|SetCollisionEnabled (Variables|Default|GetSphereComponent) "NoCollision")))

(event Custom|SpawnEmitter
  (Variables|Default|SetFireIsOn true)
  (bind _returnvalue (Effects|SpawnEmitteratLocation "/Game/Realistic_Starter_VFX_Pack_Vol2/Particles/Explosion/P_Explosion_Big_A.P_Explosion_Big_A" (Variables|Default|GetSweep%20Result%20Location)))
  (bind _returnvalue_2 (Effects|SpawnEmitteratLocation "/Game/Realistic_Starter_VFX_Pack_Vol2/Particles/Fire/P_Fire_Big.P_Fire_Big" (Variables|Default|GetSweep%20Result%20Location)))
  (Utilities|FlowControl|Delay (Math|Random|RandomFloatinRange 6.0 9.0))
  (Components|DestroyComponent _returnvalue)
  (Components|DestroyComponent _returnvalue_2)
  (Actor|DestroyActor))

(event EventBeginPlay
  (Transformation|SetActorRotation (Math|Rotator|MakeRotfromX (Variables|/Script/Engine.MovementComponent|GetVelocity (Variables|Default|GetProjectileMovementComp))))
  (Variables|Default|SetRandValue (Math|Random|RandomFloatinRange -2.0 2.0)))

(event EventTick
  (params (DeltaSeconds :type Float%20%28single-precision%29))
  (bind _randvalue (Variables|Default|GetRandValue))
  (bind _sweep_result_location (Variables|Default|GetSweep%20Result%20Location))
  (Utilities|FlowControl|Sequence
    (:then_0
      (Class|Actor|AddActorWorldRotation (Math|Rotator|MakeRotator _randvalue _randvalue _randvalue)))
    (:then_1
      (if (Variables|Default|GetFireIsOn)
        (bind _outhits (Collision|MultiSphereTraceForObjects _sweep_result_location _sweep_result_location 3e+02 (Utilities|Array|MakeArray "ObjectTypeQuery3") false 0 "None"))
        (for _array_element _outhits
          (bind _returnvalue (Collision|LineTraceByChannel (Transformation|GetActorLocation (.hitactor _array_element)) (Variables|Default|GetSweep%20Result%20Location) "TraceTypeQuery1" false (Utilities|Array|MakeArray (.hitactor _array_element)) "None"))
          (if (not _returnvalue)
            (GameplayEffects|ApplyGameplayEffectToSelf :self (Ability|GetAbilitySystemComponent (.hitactor _array_element)) :GameplayEffectClass "/Game/GameplayEffects/GE_CharacterFireDamage.GE_CharacterFireDamage_C")))))))

(fn ConstructionScript)